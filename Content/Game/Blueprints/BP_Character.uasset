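; BP_Character is a character Blueprint that shows the HUB widget and keeps its health display updated.
; On BeginPlay it creates WBP_HUB, stores the reference and adds it to the viewport.
; On AnyDamage, if that widget is valid, it passes current and default health from HealthComponent to UpdateHealth and prints the current health.
; The graph only reads health and does not apply damage itself.
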(event `self.ReceiveBeginPlay`
  (bind _returnvalue (`|CreateWidget` "/Game/Game/Widget/WBP_HUB.WBP_HUB_C"))
  (bind _output_get (set `self.HUBRef` _returnvalue))
  (`UserWidget.AddToViewport` _output_get 0))

(event `self.ReceiveAnyDamage`
  (params (Damage :type "Float (single-precision)") (DamageType :type "DamageType Object Reference") (InstigatedBy :type "Controller Object Reference") (DamageCauser :type "Actor Object Reference"))
  (bind _healthcomponent (`self.HealthComponent`))
  (bind _health (`HealthComponent.Health` _healthcomponent))
  (bind _hubref (`self.HUBRef`)
    (:`then`
      (`/Game/Game/Widget/WBP_HUB.UpdateHealth` _hubref _health (`HealthComponent.DefaultHealth` _healthcomponent))
      (`KismetSystemLibrary.PrintString` (`KismetStringLibrary.Conv_DoubleToString` _health)))
    (:`else`)))

(fn `UserConstructionScript`)