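; BP_Stimpack is a pickup that gives the collecting BP_Character a temporary 1.5x walk speed boost.
; PickUpComponent's OnPickUp saves the current max speed, applies the boost, hides the Niagara effect and starts a one-shot timer.
; When the timer fires, ReturnDefault restores the saved speed and destroys the actor.
; The IsSpeedBoosted guard is checked on pickup but never set true.
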(event `self.ReceiveBeginPlay`
  (set `self.bIsSpeedBoosted` false)
  (set `self.ActiveTime` 3.0))

(event `self.PickUpComponent.OnPickUp`
  (params (PickUpCharacter :type "OutbreakCharacter Object Reference"))
  (bind _asbp_character (cast `/Game/Game/Blueprints/BP_Character` PickUpCharacter))
  (if (not (`self.bIsSpeedBoosted`))
    (bind _charactermovement (`Character.CharacterMovement` _asbp_character))
    (bind _returnvalue (`MovementComponent.GetMaxSpeed` _charactermovement))
    (set `self.DefaultSpeed` _returnvalue)
    (set `CharacterMovementComponent.MaxWalkSpeed` (* _returnvalue 1.5) _charactermovement)
    (`SceneComponent.SetVisibility` (`self.Niagara`) false false)
    (`KismetSystemLibrary.K2_SetTimerDelegate` (delegate `Return Default`) (`self.ActiveTime`))))

(event `Return Default`
  (set `CharacterMovementComponent.MaxWalkSpeed` (`self.DefaultSpeed`) (`Character.CharacterMovement` (stale `self.PickUpComponent.OnPickUp` _asbp_character)))
  (`self.K2_DestroyActor`))

(fn `UserConstructionScript`)