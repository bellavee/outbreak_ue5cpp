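; BP_Rambo is a pickup that grants a rifle-carrying character five seconds of unlimited ammo.
; On pickup, it searches the character's attached actors for WeaponPickUp weapons and switches off the ammo limit on their WeaponComponent.
; It hides its Niagara effect but stays alive through a Delay, then restores the ammo limit and destroys itself.
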(event `self.PickUpComponent.OnPickUp`
  (params (PickUpCharacter :type "OutbreakCharacter Object Reference"))
  (if (`OutbreakCharacter.bHasRifle` PickUpCharacter)
    (for _array_element (`self.GetAttachedActors` PickUpCharacter true false)
      (bind _asweapon_pick_up (cast `WeaponPickUp` _array_element))
      (`/Engine/EditorBlueprintResources/StandardMacros.IsValid` _asweapon_pick_up
        (:`Is Valid`
          (bind _weaponcomponent (`WeaponPickUp.WeaponComponent` _asweapon_pick_up))
          (set `TP_WeaponComponent.bIsLimitAmmo` false _weaponcomponent)
          (`SceneComponent.SetVisibility` (`self.Niagara`) false false)
          (`KismetSystemLibrary.Delay` 5.0)
          (set `TP_WeaponComponent.bIsLimitAmmo` true _weaponcomponent)
          (`self.K2_DestroyActor`))))))

(fn `UserConstructionScript`)