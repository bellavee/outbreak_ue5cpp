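; BP_ZombieBase is a zombie enemy that chases the player and deals contact damage.
; Every Tick it issues an AI MoveTo targeting player character 0.
; A capsule hit on a BP_Character applies BaseDamage and sets a cooldown flag that blocks further hits.
; After the AttackCoolDown delay it only prints a debug message; the flag is cleared only on BeginPlay, so damage lands once.
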(event `self.ReceiveBeginPlay`
  (set `self.bIsAttackingCoolDown` false))

(event `self.ReceiveTick`
  (params (DeltaSeconds :type "Float (single-precision)"))
  (`|AIMoveTo` self (200.0 200.0 0.0) (`GameplayStatics.GetPlayerCharacter` 0) 5.08))

(event `self.CapsuleComponent.OnComponentHit`
  (params (HitComponent :type "PrimitiveComponent Object Reference") (OtherActor :type "Actor Object Reference") (OtherComp :type "PrimitiveComponent Object Reference") (NormalImpulse :type "Vector Structure") (Hit :type "HitResult Structure (by ref)"))
  (bind _asbp_character (cast `/Game/Game/Blueprints/BP_Character` OtherActor))
  (if (not (`self.bIsAttackingCoolDown`))
    (`GameplayStatics.ApplyDamage` _asbp_character (`self.BaseDamage`))
    (set `self.bIsAttackingCoolDown` true)
    (`KismetSystemLibrary.Delay` (`self.AttackCoolDown`))
    (`KismetSystemLibrary.PrintString` "Zombie hits")))

(fn `UserConstructionScript`)