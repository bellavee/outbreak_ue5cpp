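; BP_Mud is a mud obstacle that slows a BP_Character while it is in contact.
; OnGet stores the character's current max speed in DefaultSpeed and sets MaxWalkSpeed to three quarters of it.
; OnOut writes DefaultSpeed back to MaxWalkSpeed.
; The saved speed is a single variable on the obstacle, shared by every character that triggers it.
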(event `self.OnGet`
  (params (OverlappedComp :type "PrimitiveComponent Object Reference") (OtherActor :type "Actor Object Reference") (OtherComp :type "PrimitiveComponent Object Reference") (OtherBodyIndex :type Integer) (bFromSweep :type Boolean) (SweepResult :type "HitResult Structure (by ref)"))
  (bind _asbp_character (cast `/Game/Game/Blueprints/BP_Character` OtherActor))
  (bind _charactermovement (`Character.CharacterMovement` _asbp_character))
  (bind _returnvalue (`MovementComponent.GetMaxSpeed` _charactermovement))
  (set `self.DefaultSpeed` _returnvalue)
  (set `CharacterMovementComponent.MaxWalkSpeed` (* _returnvalue 0.75) _charactermovement))

(event `self.OnOut`
  (params (OverlappedComp :type "PrimitiveComponent Object Reference") (OtherActor :type "Actor Object Reference") (OtherComp :type "PrimitiveComponent Object Reference") (OtherBodyIndex :type Integer))
  (bind _asbp_character (cast `/Game/Game/Blueprints/BP_Character` OtherActor))
  (set `CharacterMovementComponent.MaxWalkSpeed` (`self.DefaultSpeed`) (`Character.CharacterMovement` _asbp_character)))

(fn `UserConstructionScript`)